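; Base enemy for a retro first-person game, drawn as a billboard flipbook sprite with eight-directional animation, that runs a behavior tree on BeginPlay.
; Each tick it yaws the sprite toward the camera, then, unless dead or paused, computes its facing angle to the player.
; Dot products give angle and visible side, selecting one of five facings with left/right variants.
; Velocity picks run or idle flipbooks; the angle is debug-printed.
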(event EventBeginPlay
  (bind _asbp_retro_pfsenemy_ai (Utilities|Casting|CastToBP_RetroPFSEnemyAI (Pawn|GetController)))
  (AI|RunBehaviorTree _asbp_retro_pfsenemy_ai (Variables|Default|GetBehavior%20Tree)))

(event EventTick
  (params (DeltaSeconds :type Float%20%28single-precision%29))
  (Utilities|SpriteFacePlayer
    (:Out
      (if (not (or (Variables|Default|GetIs%20Dead) (Variables|Default|GetPause%20Angle%20Calculation)))
        (Utilities|GetEnemyAngle
          (:Out
            (Utilities|CheckifWalcking
              (:Out
                (Utilities|CalculateFlipbook)))))))))

(fn ConstructionScript)

(fn SetFlipbook
  (params (Walking :type Paper%20Flipbook%20Object%20Reference) (Idle :type Paper%20Flipbook%20Object%20Reference))
  (bind _enemy (Variables|Default|GetEnemy))
  (if (Variables|Default|GetIs%20Walking)
    (Sprite|SetFlipbook _enemy Walking)
    (else
      (Sprite|SetFlipbook _enemy Idle))))
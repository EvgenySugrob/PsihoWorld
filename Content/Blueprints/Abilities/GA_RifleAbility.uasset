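; Gameplay ability that fires the player's rifle as a hitscan shot.
; FireWeapon lazily caches the owning first-person character and its child-actor rifle, then calls ShotRifle on the rifle.
; A Visibility line trace starts at the camera, and any RetroFPSCharacter hit receives ApplyEffect with the player as attacker.
; The trace end is camera forward times WeaponRange, without adding the camera location.
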(event EventFireWeapon
  (bind _player_rifle_weapon_component (Variables|Default|GetPlayer%20Rifle%20Weapon%20Component))
  ;[1 1 1] Fire Rifle
  (CallFunction|GetPlayer)
  (CallFunction|GetWeapon)
  (Utilities|IsValid _player_rifle_weapon_component
    (:Is%20Valid
      (Default|ShotRifle _player_rifle_weapon_component)
      (bind _actor (CallFunction|GetLineTrace))
      (bind _asretro_fpscharacter (Utilities|Casting|CastToRetroFPSCharacter _actor))
      (CallFunction|ApplyEffect (Variables|Default|GetPlayer) _asretro_fpscharacter))))

(fn GetPlayer
  (Utilities|IsValid (Variables|Default|GetPlayer)
    (:Is%20Valid
      _)
    (:Is%20Not%20Valid
      (bind _asbp_first_person_character (Utilities|Casting|CastToBP_FirstPersonCharacter (.owneractor (Ability|GetActorInfo))))
      (Variables|Default|SetPlayer _asbp_first_person_character)))
  (return))

(fn GetWeapon
  (Utilities|IsValid (Variables|Default|GetPlayer%20Rifle%20Weapon%20Component)
    (:Is%20Valid
      _)
    (:Is%20Not%20Valid
      (bind _asbp_rifle (Utilities|Casting|CastToBP_Rifle (Variables|/Script/Engine.ChildActorComponent|GetChildActor (Variables|/Game/FirstPerson/Blueprints/BP_FirstPersonCharacter.BP_FirstPersonCharacter_C|GetWeapon (Variables|Default|GetPlayer)))))
      (Variables|Default|SetPlayer%20Rifle%20Weapon%20Component _asbp_rifle)))
  (return))

(fn GetLineTrace
  (bind _player (Variables|Default|GetPlayer))
  (bind _firstpersoncamera (Variables|/Game/FirstPerson/Blueprints/BP_FirstPersonCharacter.BP_FirstPersonCharacter_C|GetFirstPersonCamera _player))
  (bind _outhit (Collision|LineTraceByChannel (Transformation|GetWorldLocation _firstpersoncamera) (* (Math|Vector|GetForwardVector (Transformation|GetWorldRotation _firstpersoncamera)) (Variables|Default|GetWeapon%20Range)) "TraceTypeQuery1" false 0 "None"))
  (Utilities|IsValid (.HitActor (Collision|BreakHitResult _outhit))
    (:Is%20Valid
      (return (.HitActor (Collision|BreakHitResult _outhit))))))
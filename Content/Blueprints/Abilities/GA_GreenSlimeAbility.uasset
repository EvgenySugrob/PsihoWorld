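; Gameplay ability that gives the green slime enemy a ranged hitscan attack against the retro FPS player character.
; On FireWeapon it caches the owning BP_GreenSlime, then traces the Visibility channel forward from its capsule over WeaponRange.
; If the hit actor is a RetroFPSCharacter, it calls ApplyEffect with the slime as attacker.
; The trace leaves debug drawing on for a timed duration.
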(event Ability|EventActivateAbility
  (|CallParentFunction) ; This node is disabled and will not be called.\nDrag off pins to build functionality.
)

(event Ability|EventOnEndAbility
  (params (bWasCancelled :type Boolean))
  (|CallParentFunction bWasCancelled) ; This node is disabled and will not be called.\nDrag off pins to build functionality.
)

(event EventFireWeapon
  (CallFunction|GetEnemy)
  (bind _actor (CallFunction|GetLineTrace))
  (bind _asretro_fpscharacter (Utilities|Casting|CastToRetroFPSCharacter _actor))
  (CallFunction|ApplyEffect (Variables|Default|GetGreen%20Slime) _asretro_fpscharacter))

(fn GetLineTrace
  (bind _green_slime (Variables|Default|GetGreen%20Slime))
  (bind _capsulecomponent (Variables|/Script/Engine.Character|GetCapsuleComponent _green_slime))
  (bind _returnvalue (Transformation|GetWorldLocation _capsulecomponent))
  (bind _outhit (Collision|LineTraceByChannel _returnvalue (+ _returnvalue (* (Math|Vector|GetForwardVector (Transformation|GetWorldRotation _capsulecomponent)) (Variables|Default|GetWeapon%20Range))) "TraceTypeQuery1" false 0 "ForDuration" true "(R=1.000000,G=0.000000,B=0.000000,A=1.000000)" "(R=0.000000,G=1.000000,B=0.000000,A=1.000000)" 1e+01))
  (Utilities|IsValid (.HitActor (Collision|BreakHitResult _outhit))
    (:Is%20Valid
      (return (.HitActor (Collision|BreakHitResult _outhit))))))

(fn GetEnemy
  (Utilities|IsValid (Variables|Default|GetGreen%20Slime)
    (:Is%20Valid
      _)
    (:Is%20Not%20Valid
      (bind _asbp_green_slime (Utilities|Casting|CastToBP_GreenSlime (.owneractor (Ability|GetActorInfo))))
      (Variables|Default|SetGreen%20Slime _asbp_green_slime)))
  (return))
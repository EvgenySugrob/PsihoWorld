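; Retro character Blueprint that reacts to damage and death through Gameplay Ability System attributes.
; TakeDamage takes gameplay cue data, prints debug health and armor readouts, and reports the hit to AI damage sensing with the effect's instigator and location.
; HealthCheck then tests whether an attribute, presumably health, is at or below zero and, if so, calls KillCharacter, which is an empty event here.
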(event Custom|Take%20Damage
  (params (Cue%20Data :type Gameplay%20Cue%20Parameters%20Structure))
  (bind (_normalizedmagnitude _rawmagnitude _effectcontext _matchedtagname _originaltag _aggregatedsourcetags _aggregatedtargettags _location) (Ability|GameplayCue|BreakGameplayCueParameters Cue%20Data))
  (bind _abilitysystemcomponent (Variables|Default|GetAbilitySystemComponent))
  (Development|PrintString (Utilities|String|Append "Health: " (Utilities|String|ToString(Float) (.ReturnValue (Ability|Attribute|GetFloatAttributefromAbilitySystemComponent _abilitysystemcomponent "(AttributeName=\"Health\",Attribute=/Script/PsihoWorld.RetroFPSAttributeSet:Health,AttributeOwner=/Script/CoreUObject.Class'\"/Script/PsihoWorld.RetroFPSAttributeSet\"')"))) "Armor: " (Utilities|String|ToString(Float) (.ReturnValue (Ability|Attribute|GetFloatAttributefromAbilitySystemComponent _abilitysystemcomponent "(AttributeName=\"Armor\",Attribute=/Script/PsihoWorld.RetroFPSAttributeSet:Armor,AttributeOwner=/Script/CoreUObject.Class'\"/Script/PsihoWorld.RetroFPSAttributeSet\"')")))) true true "(R=0.000000,G=0.660000,B=1.000000,A=1.000000)" 6e+01)
  (Class|AISenseDamage|ReportDamageEvent self (Class|AbilitySystemBlueprintLibrary|EffectContextGetInstigatorActor _effectcontext) 0.0 _location "0, 0, 0" "None")
  (Development|PrintString (Utilities|String|Append (Utilities|GetDisplayName self) "'s current Health" (Utilities|String|ToString(Float) (.ReturnValue (Ability|Attribute|GetFloatAttributefromAbilitySystemComponent (Variables|Default|GetAbilitySystemComponent) "(AttributeName=\"Health\",Attribute=/Script/PsihoWorld.RetroFPSAttributeSet:Health,AttributeOwner=/Script/CoreUObject.Class'\"/Script/PsihoWorld.RetroFPSAttributeSet\"')")))) true true "(R=0.000000,G=0.660000,B=1.000000,A=1.000000)" 6e+01)
  (if (CallFunction|HealthCheck)
    (CallFunction|KillCharacter)))

(event Custom|Kill%20Character)

(fn ConstructionScript)

(fn HealthCheck
  (return (<= (.ReturnValue (Ability|Attribute|GetFloatAttributefromAbilitySystemComponent (Variables|Default|GetAbilitySystemComponent) "(AttributeName=\"Health\",Attribute=/Script/PsihoWorld.RetroFPSAttributeSet:Health,AttributeOwner=/Script/CoreUObject.Class'\"/Script/PsihoWorld.RetroFPSAttributeSet\"')")) 0.0)))
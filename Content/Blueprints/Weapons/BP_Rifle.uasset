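; BP_Rifle is a rifle weapon Blueprint that drives the weapon's flipbook visuals.
; Initializing the weapon sets its flipbook to idle and makes it visible.
; Firing switches to the fire flipbook, waits for that flipbook's length, then returns to idle.
; The construction script only calls the parent's, so the rest of the weapon logic is not defined here.
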(event Custom|Shot%20Rifle
  (bind _weaponflipbook (Variables|Default|GetWeaponFlipbook))
  ;[0 0 0] Pistol Fire Animation
  (Sprite|SetFlipbook _weaponflipbook (Variables|Default|GetFire%20Rifle))
  (Utilities|FlowControl|Delay (Class|PaperFlipbookComponent|GetFlipbookLength _weaponflipbook))
  (Sprite|SetFlipbook (Variables|Default|GetWeaponFlipbook) (Variables|Default|GetIdle%20Flipbook)))

(event EventInitializeWeapon
  ;[0 0 0] Equip Weapon
  (Sprite|SetFlipbook (Variables|Default|GetWeaponFlipbook) (Variables|Default|GetIdle%20Flipbook))
  (Development|SetHiddeninGame (Variables|Default|GetWeaponFlipbook) false false))

(fn ConstructionScript
  (|CallParentFunction))
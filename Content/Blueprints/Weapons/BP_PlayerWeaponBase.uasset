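; BP_PlayerWeaponBase is the base player weapon, displayed as a flipbook sprite.
; A SceneCaptureComponent2D is restricted to rendering only that flipbook, and the flipbook's starting relative location is cached on BeginPlay.
; InitializeWeapon clears the flipbook and hides it in game.
; WeaponBobbing plays the WeaponBob sequence while moving, then stops it and interpolates the sprite back toward its cached position when idle.
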(event Custom|Weapon%20Bobbing
  (params (Is%20Move :type Boolean) (Delta%20Time :type Float%20%28double-precision%29))
  (bind _weapon_bob (Variables|Default|GetWeapon%20Bob))
  (bind _weaponflipbook (Variables|Default|GetWeaponFlipbook))
  (bind _sequenceplayer (Variables|/Script/ActorSequence.ActorSequenceComponent|GetSequencePlayer _weapon_bob))
  (if Is%20Move
    (Sequencer|Player|Play _sequenceplayer :!class /Script/MovieScene.MovieSceneSequencePlayer)
    (else
      (Sequencer|Player|Stop _sequenceplayer :!class /Script/MovieScene.MovieSceneSequencePlayer)
      (Transformation|SetRelativeLocation _weaponflipbook (Math|Interpolation|VInterpTo (Variables|/Script/Engine.SceneComponent|GetRelativeLocation _weaponflipbook) (Variables|Default|GetWeapon%20Position) Delta%20Time 15.0) false false))))

(event EventBeginPlay
  (Rendering|SceneCapture|ShowOnlyComponent (Variables|Default|GetSceneCaptureComponent2D) (Variables|Default|GetWeaponFlipbook))
  (Variables|Default|SetWeapon%20Position (Variables|/Script/Engine.SceneComponent|GetRelativeLocation (Variables|Default|GetWeaponFlipbook))))

(event Collision|EventActorBeginOverlap
  (params (OtherActor :type Actor%20Object%20Reference)))

(event EventTick
  (params (DeltaSeconds :type Float%20%28single-precision%29)))

(event EventInitializeWeapon
  (bind _weaponflipbook (Variables|Default|GetWeaponFlipbook))
  (Sprite|SetFlipbook _weaponflipbook)
  (Development|SetHiddeninGame _weaponflipbook true false))

(fn ConstructionScript)